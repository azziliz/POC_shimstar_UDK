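; A physics-driven pawn Blueprint that continuously pushes itself along its facing direction.
; Each Tick adds the actor's forward vector, scaled by Vitesse (speed), to the StaticMesh's linear velocity, without scaling by delta time.
; The inputAcceleration axis feeds AddAcceleration, whose body is not shown here.
; The moveUp axis does nothing, and a right-vector strafe push is left disconnected.
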(event `self.ReceiveBeginPlay`)

(event `self.ReceiveActorBeginOverlap`
  (params (OtherActor :type "Actor Object Reference")))

(event `self.ReceiveTick`
  (params (DeltaSeconds :type "Float (single-precision)"))
  (`PrimitiveComponent.SetPhysicsLinearVelocity` (`self.StaticMesh`) (* (`KismetMathLibrary.GetForwardVector` (`self.K2_GetActorRotation`)) (`self.vitesse`)) true "None"))

(event `InputAxis|inputAcceleration`
  (params (AxisValue :type "Float (single-precision)"))
  (`self.addAcceleration` AxisValue))

(event `InputAxis|moveUp`
  (params (AxisValue :type "Float (single-precision)")))

(fn `UserConstructionScript`)